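; Homing meteor projectile that explodes on impact and passes rovers caught in its blast sphere to BP_OurGM for respawn.
; On the server, Setup launches it at a target component and sets a replicated rotation that orients the particle trail through OnRep.
; It detonates on overlapping a non-meteor, or when a delayed looping timer finds it barely moving near the target.
; Detonation runs once, spawning explosion effects and destroying the actor.
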(event OnComponentBeginOverlap(Sphere)
  (params (OverlappedComponent :type Primitive%20Component%20Object%20Reference) (OtherActor :type Actor%20Object%20Reference) (OtherComp :type Primitive%20Component%20Object%20Reference) (OtherBodyIndex :type Integer) (bFromSweep :type Boolean) (SweepResult :type Hit%20Result%20Structure%20%28by%20ref%29))
  (bind _returnvalue (Transformation|GetActorLocation))
  (Networking|SwitchHasAuthority
    (:Authority
      (if (!= (Utilities|GetClass OtherActor) "BP_Meteor_C")
        (if (not (Variables|Default|GetDestroy))
          (Variables|Default|SetDestroy true)
          (bind _asbp_our_gm (Utilities|Casting|CastToBP_OurGM (Game|GetGameMode)))
          (Default|RoverstoRespawnAfterMeteor _asbp_our_gm (Collision|GetOverlappingActors (Variables|Default|GetSphere1) "/Game/CustomVehicle/ParentRover.ParentRover_C" :!class /Script/Engine.PrimitiveComponent))
          (Effects|SpawnEmitteratLocation "/Game/VFX_Toolkit_V1/ParticleSystems/356Days/Par_Meteora_Explode_01.Par_Meteora_Explode_01" _returnvalue "0, 0, 0" (Transformation|GetActorScale3D))
          (Audio|SpawnSoundatLocation "/Game/Lewin/Sounds/Meteor/MeteorHit.MeteorHit" _returnvalue "0, 0, 0" 1.0 1.0 0.0 "/Game/Lewin/Sounds/Meteor/MeteorAttenuation.MeteorAttenuation" 0)
          (Actor|DestroyActor))))))

(event Custom|Setup
  (params (NewParam :type Scene%20Component%20Object%20Reference) (Rotation :type Rotator) (Initial%20Speed :type Float%20%28single-precision%29))
  (bind (_roll _pitch _yaw) (Math|Rotator|BreakRotator Rotation))
  (bind _projectilemovement (Variables|Default|GetProjectileMovement))
  (bind _projectilemovement_2 (Variables|Default|GetProjectileMovement))
  (Networking|SwitchHasAuthority
    (:Authority
      (Variables|/Script/Engine.ProjectileMovementComponent|SetInitialSpeed _projectilemovement_2 Initial%20Speed)
      (Variables|/Script/Engine.ProjectileMovementComponent|SetMaxSpeed _projectilemovement_2 Initial%20Speed)
      (Components|Activation|Activate _projectilemovement_2 false)
      (Variables|Default|SetRotation (Math|Rotator|MakeRotator _roll (+ _pitch 9e+01) _yaw))
      (bind _output_get (Variables|Default|SetTargetComponent NewParam))
      (Variables|/Script/Engine.ProjectileMovementComponent|SetHomingTargetComponent _projectilemovement _output_get)
      (Variables|/Script/Engine.ProjectileMovementComponent|SetbIsHomingProjectile _projectilemovement true)
      (Utilities|FlowControl|Delay 3.0)
      (Utilities|Time|SetTimerbyEvent (delegate Custom|CustomEvent_0) 0.1 true))))

(event Custom|CustomEvent_0
  (bind _returnvalue (Transformation|GetActorLocation))
  (bind _returnvalue_2 (Transformation|GetActorLocation))
  (if (and (Math|Vector|Equal(Vector) _returnvalue (Variables|Default|GetPreLoc) 2e+02) (< (Math|Vector|Distance(Vector) (Transformation|GetWorldLocation (Variables|Default|GetTargetComponent)) (Transformation|GetActorLocation)) 6e+02))
    (if (not (Variables|Default|GetDestroy))
      (Variables|Default|SetDestroy true)
      (bind _asbp_our_gm (Utilities|Casting|CastToBP_OurGM (Game|GetGameMode)))
      (Default|RoverstoRespawnAfterMeteor _asbp_our_gm (Collision|GetOverlappingActors (Variables|Default|GetSphere1) "/Game/CustomVehicle/ParentRover.ParentRover_C" :!class /Script/Engine.PrimitiveComponent))
      (Effects|SpawnEmitteratLocation "/Game/VFX_Toolkit_V1/ParticleSystems/356Days/Par_Meteora_Explode_01.Par_Meteora_Explode_01" _returnvalue_2 "0, 0, 0" (Transformation|GetActorScale3D))
      (Audio|SpawnSoundatLocation "/Game/Lewin/Sounds/Meteor/MeteorHit.MeteorHit" _returnvalue_2 "0, 0, 0" 1.0 1.0 0.0 "/Game/Lewin/Sounds/Meteor/MeteorAttenuation.MeteorAttenuation" 0)
      (Actor|DestroyActor))
    (else
      (Variables|Default|SetPreLoc _returnvalue))))

(fn ConstructionScript)

(fn OnRepRotation
  (Transformation|SetWorldRotation (Variables|Default|GetParticleSystem) (Variables|Default|GetRotation) false false))