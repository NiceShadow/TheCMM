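; BP_NewMenuPC is a menu player controller that sets up the menu UI and automatically starts hosting a game when Steam is available.
; On BeginPlay it has the FriendsIntance game instance run CreateWB, shows the cursor and switches to UI-only input.
; After short delays and a Steam subsystem check, it calls HostLoadGame on that instance as a new host, using hardcoded "test" names.
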(event EventBeginPlay
  (bind _asfriends_intance (Utilities|Casting|CastToFriendsIntance (Game|GetGameInstance))
    (:then
      (Default|CreateWB _asfriends_intance))
    (:CastFailed
      _))
  (Variables|Default|SetbShowMouseCursor true)
  (Input|SetInputModeUIOnly self 0 "DoNotLock")
  (Utilities|FlowControl|Delay 0.5)
  (if (Class|AdvancedSessionsLibrary|HasOnlineSubsystem "STEAM")
    (Utilities|FlowControl|Delay 1.4)
    (bind _asfriends_intance_2 (Utilities|Casting|CastToFriendsIntance (Game|GetGameInstance)))
    (Default|HostLoadGame _asfriends_intance_2 (Game|GetPlayerController 0) "test" (Utilities|Struct|MakeSaveGameSlot_Structure "test") true)))

(fn ConstructionScript)