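; BenchmarkChecker is an actor that runs a timed frame-rate benchmark as it flies through the level.
; BeginPlay teleports it to a fixed start point, then uses delays to open a measurement window, rotate the actor midway and close the window.
; While measuring, Tick drives FloatingPawnMovement along world X and accumulates truncated per-frame FPS from delta time.
; The average is then printed on screen as the result.
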(event EventTick
  (params (DeltaSeconds :type Float%20%28single-precision%29))
  (if (Variables|Default|Getstart)
    (Class|PawnMovementComponent|AddInputVector (Variables|Default|GetFloatingPawnMovement) "1.000000, 0, 0" false)
    (Math|Integer|IncrementInt (Variables|Default|GetCounted)
      (:%20%20
        (Variables|Default|SetTotal (+ (Math|Float|Truncate (/ 1.0 DeltaSeconds)) (Variables|Default|GetTotal)))))))

(event EventBeginPlay
  (Utilities|FlowControl|Delay 0.2)
  (Transformation|SetActorLocation "-3000.000000,16000.000000,-21000.000000" false false)
  (Utilities|FlowControl|Delay 6.0)
  (Variables|Default|Setstart true)
  (Utilities|FlowControl|Delay 5.0)
  (Transformation|SetActorRotation "0,90.000000, 0")
  (Utilities|FlowControl|Delay 5.0)
  (Variables|Default|Setstart false)
  (Utilities|FlowControl|Delay 0.4)
  (Development|PrintString (Utilities|String|Append "Result    " (Utilities|String|ToString(Integer) (/ (Variables|Default|GetTotal) (Variables|Default|GetCounted)))) true true "(R=1.000000,G=0.838870,B=0.000000,A=1.000000)" 15.0))

(fn ConstructionScript)