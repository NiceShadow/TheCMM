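; BP_TerminalInstances spawns instanced meshes at runtime to match the placed terminal and HQ computer actors.
; On BeginPlay it loops over every BP_Terminal, adding a Special or Driving instance by its speciality toggle, turned 180 degrees in yaw, plus a scaled-down Monitor instance at its MonitorLoc.
; It then adds a very slightly shrunken Computers instance at each HQ_Computer_full, leaving the source actors untouched.
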(event EventBeginPlay
  (bind _outactors (Actor|GetAllActorsOfClass "/Game/Lewin/Blueprints/BP_Terminal.BP_Terminal_C"))
  (for _array_element _outactors
    (Class|InstancedStaticMeshComponent|AddInstanceWorldSpace (select (Variables|/Game/Lewin/Blueprints/BP_Terminal.BP_Terminal_C|GetTerminalSpecialityToggler _array_element) (Variables|Default|GetSpecial) (Variables|Default|GetDriving)) (Math|Transform|MakeTransform (Transformation|GetActorLocation _array_element) (Math|Rotator|MakeRotator (.Roll (Math|Rotator|BreakRotator (Transformation|GetActorRotation _array_element))) (.Pitch (Math|Rotator|BreakRotator (Transformation|GetActorRotation _array_element))) (+ (.Yaw (Math|Rotator|BreakRotator (Transformation|GetActorRotation _array_element))) 1.8e+02))))
    (Class|InstancedStaticMeshComponent|AddInstanceWorldSpace (Variables|Default|GetMonitor) (Math|Transform|MakeTransform (.Location (Math|Transform|BreakTransform (Transformation|GetWorldTransform (Variables|/Game/Lewin/Blueprints/BP_Terminal.BP_Terminal_C|GetMonitorLoc _array_element)))) (.Rotation (Math|Transform|BreakTransform (Transformation|GetWorldTransform (Variables|/Game/Lewin/Blueprints/BP_Terminal.BP_Terminal_C|GetMonitorLoc _array_element)))) "0.900000,0.900000,0.900000")))
  (bind _outactors_2 (Actor|GetAllActorsOfClass "/Game/Balduin/HQmeshes/HQ_Computer_full.HQ_Computer_full_C"))
  (for _array_element_2 _outactors_2
    (Class|InstancedStaticMeshComponent|AddInstanceWorldSpace (Variables|Default|GetComputers) (Math|Transform|MakeTransform (Transformation|GetActorLocation _array_element_2) (Transformation|GetActorRotation _array_element_2) (Math|Conversions|ToVector(Float) (Math|Float|MakeLiteralFloat 0.999))))))

(fn ConstructionScript)