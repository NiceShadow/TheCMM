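; Player controller for the menu, handling keyboard control of the load-game screen and relaying host requests.
; Up, Down, Enter and Delete select, load or delete save entries through BP_MenuHUD's menu widget while that screen is open.
; BeginPlay shows the cursor, sets Game-and-UI input, issues an FPS-cap console command and destroys any session.
; Host and SetSGSlots forward session and save-slot data to the FriendsIntance game instance.
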(event Custom|Host
  (params (LanName :type String) (SaveGameSlot_Structure :type Save%20Game%20Slot%20Structure%20Structure%20%28by%20ref%29) (Host%20New%20Game :type Boolean))
  (bind _asfriends_intance (Utilities|Casting|CastToFriendsIntance (Game|GetGameInstance)))
  (Default|HostLoadGame _asfriends_intance self LanName SaveGameSlot_Structure Host%20New%20Game))

(event Custom|Set%20SG%20Slots
  (params (AllSG_Slots :type Array%20of%20Save%20Game%20Slot%20Structure%20Structures))
  (bind _asfriends_intance (Utilities|Casting|CastToFriendsIntance (Game|GetGameInstance)))
  (Default|SetSGSlots _asfriends_intance AllSG_Slots))

(event EventBeginPlay
  (Input|SetInputModeUIOnly self 0 "DoNotLock")
  (Variables|Default|SetbShowMouseCursor true)
  (Input|SetInputModeGameandUI self 0 "DoNotLock" false)
  (Development|ExecuteConsoleCommand "t. maxfps 60" 0)
  (|DestroySession self))

(event Input|KeyboardEvents|Up
  (params (Key :type Key%20Structure))
  (:Pressed
    (bind _asbp_menu_hud (Utilities|Casting|CastToBP_MenuHUD (HUD|GetHUD)))
    (if (Variables|/Game/Server/Widgets/WB_Menu.WB_Menu_C|GetIsInLoadGameMenu? (Variables|/Game/Server/BP_MenuHUD.BP_MenuHUD_C|GetMenuRef _asbp_menu_hud))
      (Default|SelectNextLoadWidget (Variables|/Game/Server/BP_MenuHUD.BP_MenuHUD_C|GetMenuRef _asbp_menu_hud) true))))

(event Input|KeyboardEvents|Down
  (params (Key :type Key%20Structure))
  (:Pressed
    (bind _asbp_menu_hud (Utilities|Casting|CastToBP_MenuHUD (HUD|GetHUD)))
    (if (Variables|/Game/Server/Widgets/WB_Menu.WB_Menu_C|GetIsInLoadGameMenu? (Variables|/Game/Server/BP_MenuHUD.BP_MenuHUD_C|GetMenuRef _asbp_menu_hud))
      (Default|SelectNextLoadWidget (Variables|/Game/Server/BP_MenuHUD.BP_MenuHUD_C|GetMenuRef _asbp_menu_hud) false))))

(event Input|KeyboardEvents|Enter
  (params (Key :type Key%20Structure))
  (:Pressed
    (bind _asbp_menu_hud (Utilities|Casting|CastToBP_MenuHUD (HUD|GetHUD)))
    (if (Variables|/Game/Server/Widgets/WB_Menu.WB_Menu_C|GetIsInLoadGameMenu? (Variables|/Game/Server/BP_MenuHUD.BP_MenuHUD_C|GetMenuRef _asbp_menu_hud))
      (Default|Load (Variables|/Game/Server/Widgets/WB_Menu.WB_Menu_C|GetactivatedLoadWidget (Variables|/Game/Server/BP_MenuHUD.BP_MenuHUD_C|GetMenuRef _asbp_menu_hud))))))

(event Input|KeyboardEvents|Delete
  (params (Key :type Key%20Structure))
  (:Pressed
    (bind _asbp_menu_hud (Utilities|Casting|CastToBP_MenuHUD (HUD|GetHUD)))
    (if (Variables|/Game/Server/Widgets/WB_Menu.WB_Menu_C|GetIsInLoadGameMenu? (Variables|/Game/Server/BP_MenuHUD.BP_MenuHUD_C|GetMenuRef _asbp_menu_hud))
      (Default|Delete (Variables|/Game/Server/Widgets/WB_Menu.WB_Menu_C|GetactivatedLoadWidget (Variables|/Game/Server/BP_MenuHUD.BP_MenuHUD_C|GetMenuRef _asbp_menu_hud))))))

(fn ConstructionScript)