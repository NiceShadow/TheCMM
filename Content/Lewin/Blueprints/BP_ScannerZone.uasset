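; BP_ScannerZone generates random nested scanning zones with objective rocks on the server.
; It offsets each smaller circle inside the previous one, then uses vertical sphere traces to check that enough foliage instances lie within.
; Failed layouts retry in batches separated by a delay to avoid infinite loops.
; On success, it picks shuffled instances per zone and sends zone centers and objective locations to the GameMode through an event dispatcher.
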(event Custom|PendingGenerate
  ;[1 1 1] Prevent invinite loop and wait a short time before trying to generate again
  (Utilities|FlowControl|Delay (Variables|Default|GetUpdate))
  (CallFunction|GenerateRandomZones))

(event Custom|GenerateOnServer
  (params (Zones :type Array%20of%20ST%20Scanner%20Zones%20Structures))
  ;[1 1 1] Generate random scanning zones
  (CallFunction|SetupandStartGenerating Zones))

(fn ConstructionScript)

(fn CreateCircle
  (params (InSphereRadius :type Float%20%28single-precision%29) (Target :type Sphere%20Component%20Object%20Reference) (Before :type Sphere%20Component%20Object%20Reference))
  (Components|Sphere|SetSphereRadius Target InSphereRadius true)
  (Transformation|SetWorldLocation Target (+ (Transformation|GetWorldLocation Before) (* (Math|Vector|RotateVector (Math|Vector|GetForwardVector (Transformation|GetActorRotation)) (Math|Rotator|MakeRotator 0.0 0.0 (Math|Conversions|ToFloat(Integer) (Math|Random|RandomIntegerinRange 0 360)))) (Math|Random|RandomIntegerinRange 20 (Math|Float|Truncate (- (Variables|/Script/Engine.SphereComponent|GetSphereRadius Before) InSphereRadius))))) false false))

(fn ScanCircle
  (params (InSphereRadius :type Float%20%28single-precision%29) (Target :type Sphere%20Component%20Object%20Reference) (Before :type Sphere%20Component%20Object%20Reference))
  (Components|Sphere|SetSphereRadius Target InSphereRadius true)
  (Transformation|SetWorldLocation Target (+ (Transformation|GetWorldLocation Before) (* (Math|Vector|RotateVector (Math|Vector|GetForwardVector (Transformation|GetActorRotation)) (Math|Rotator|MakeRotator 0.0 0.0 (Math|Conversions|ToFloat(Integer) (Math|Random|RandomIntegerinRange 0 360)))) (Math|Random|RandomIntegerinRange 20 (Math|Float|Truncate (- (Variables|/Script/Engine.SphereComponent|GetSphereRadius Before) InSphereRadius))))) false false))

(fn TrytoGenerateRandomZone
  (Utilities|Array|Clear (Variables|Default|GetFoundZoneLocs))
  (LocalVariables|SetLocationOfBiggerCircle (Transformation|GetActorLocation))
  (for (_array_element _array_index) (Variables|Default|GetZonesRadius)
    (if (> _array_index 0)
      (LocalVariables|SetLocationOfBiggerCircle (+ (LocalVariables|GetLocationOfBiggerCircle) (* (Math|Vector|RotateVector (Math|Vector|GetForwardVector (Transformation|GetActorRotation)) (Math|Rotator|MakeRotator 0.0 0.0 (Math|Conversions|ToFloat(Integer) (Math|Random|RandomIntegerinRange 0 360)))) (Math|Random|RandomIntegerinRange (/ _array_element 2) (Math|Float|Truncate (- (Math|Conversions|ToFloat(Integer) (Utilities|Array|Get(acopy) (Variables|Default|GetZonesRadius) (- _array_index 1))) (Math|Conversions|ToFloat(Integer) _array_element))))))))
    (Utilities|Array|Clear (LocalVariables|Getc))
    (bind _outhits (Collision|MultiSphereTraceByChannel (.Start (CallFunction|GetSphereTraceLocs (LocalVariables|GetLocationOfBiggerCircle))) (.End (CallFunction|GetSphereTraceLocs (LocalVariables|GetLocationOfBiggerCircle))) (Math|Conversions|ToFloat(Integer) _array_element) "TraceTypeQuery3" false 0 "None" true "(R=1.000000,G=0.000000,B=0.000000,A=1.000000)" "(R=0.000000,G=1.000000,B=0.000000,A=1.000000)" 3e+01))
    (for _array_element_2 _outhits
      (Utilities|Array|AddUnique (LocalVariables|Getc) (.HitItem (Collision|BreakHitResult _array_element_2))))
    (Utilities|Array|Add (LocalVariables|GetAmountOfInstances) (Utilities|Array|Length (LocalVariables|Getc)))
    (Utilities|Array|Add (Variables|Default|GetFoundZoneLocs) (LocalVariables|GetLocationOfBiggerCircle)))
  (bind _output_get (LocalVariables|SetAmountOfInstancesReversed (LocalVariables|GetAmountOfInstances)))
  (Utilities|Array|Reverse _output_get)
  (for (_array_element_3 _array_index_2) (LocalVariables|GetAmountOfInstancesReversed)
    (if (>= (- _array_element_3 (LocalVariables|GetCurrentTotalAmountCount)) (Utilities|Array|Get(acopy) (Variables|Default|GetZonesObjectivesReversed) _array_index_2))
      (LocalVariables|SetCurrentTotalAmountCount (+ _array_element_3 (LocalVariables|GetCurrentTotalAmountCount)))
      (else
        (return false))))
  (return true))

(fn GenerateRandomZones
  (bind _returnvalue (Math|Random|RandomFloat))
  (bind _returnvalue_2 (Math|Random|RandomFloat))
  (bind _returnvalue_3 (Math|Random|RandomFloat))
  (bind _dev (Variables|Default|GetDev))
  (bind _scanningzoneresults (Variables|Default|GetScanningZoneResults))
  (bind _dev_2 (Variables|Default|GetDev))
  (bind _scanningzoneresults_2 (Variables|Default|GetScanningZoneResults))
  (bind (_radiuslocations _objectivelocations) (Utilities|Struct|BreakST_ScanningZoneResult _scanningzoneresults))
  (bind (_radiuslocations_2 _objectivelocations_2) (Utilities|Struct|BreakST_ScanningZoneResult _scanningzoneresults_2))
  (bind _returnvalue_4 (Math|Color|MakeColor _returnvalue_2 _returnvalue_3 _returnvalue))
  ;[1 1 1] Reset arrays
  (Utilities|Array|Clear (Variables|Default|GetObjectivesSelected))
  (bind _output_get (Variables|Default|SetZonesObjectivesReversed (Variables|Default|GetZonesAmountOfObjectives)))
  (Utilities|Array|Reverse _output_get)
  (bind _output_get_2 (Variables|Default|SetZonesRadiusReversed (Variables|Default|GetZonesRadius)))
  (Utilities|Array|Reverse _output_get_2)
  ;[1 1 1] On generating try loop repetition
  (Math|Integer|IncrementInt (LocalVariables|GetAttempts) :!label _label
    (:%20%20
      (Math|Integer|IncrementInt (Variables|Default|GetTotalAttempts)
        (:%20%20
          (bind _found (CallFunction|TrytoGenerateRandomZone))
          (if _found
            ;[1 1 1] Successful generated scanning zones
            (Development|PrintString (Utilities|String|Append "Total Attempts to generate scan zones: " (Utilities|String|ToString(Integer) (Variables|Default|GetTotalAttempts))) _dev _dev "(R=0.001346,G=1.000000,B=0.000000,A=1.000000)" 3.0)
            ;[1 1 1] Setup for next step
            (Utilities|Array|Clear (Utilities|Struct|BreakST_ScanningZoneResult (Variables|Default|GetScanningZoneResults)))
            (bind _output_get_3 (Variables|Default|SetFoundReversed (Variables|Default|GetFoundZoneLocs)))
            (Utilities|Array|Reverse _output_get_3)
            ;[1 1 1] Select random objective rocks
            (for (_array_element _array_index) (Variables|Default|GetFoundReversed)
              (Utilities|Array|Clear (LocalVariables|GetAllFound))
              (Utilities|Array|Clear (LocalVariables|GetCurrentHitItems))
              (Utilities|Array|Clear (LocalVariables|GetOneZoneIndividuals))
              (bind _outhits (Collision|MultiSphereTraceByChannel (.Start (CallFunction|GetSphereTraceLocs _array_element)) (.End (CallFunction|GetSphereTraceLocs _array_element)) (Math|Conversions|ToFloat(Integer) (Utilities|Array|Get(acopy) (Variables|Default|GetZonesRadiusReversed) _array_index)) "TraceTypeQuery3" true 0 "None" true _returnvalue_4 _returnvalue_4 3e+01))
              (bind _output_get_4 (Variables|Default|SetCurrentResults _outhits))
              (for _array_element_2 _output_get_4
                (Utilities|Array|AddUnique (LocalVariables|GetOneZoneIndividuals) (.HitItem (Collision|BreakHitResult _array_element_2))))
              (for _array_element_3 (LocalVariables|GetOneZoneIndividuals)
                (if (not (Utilities|Array|ContainsItem (LocalVariables|GetAlreadyTraced) _array_element_3))
                  (if (not (Utilities|Array|ContainsItem (Variables|Default|GetObjectivesSelected) _array_element_3))
                    (Utilities|Array|Add (LocalVariables|GetCurrentHitItems) _array_element_3))))
              (Utilities|Array|Shuffle (LocalVariables|GetCurrentHitItems))
              (for _array_element_4 (Variables|Default|GetCurrentResults)
                (Utilities|Array|Add (LocalVariables|GetAlreadyTraced) (.HitItem (Collision|BreakHitResult _array_element_4))))
              (Utilities|Array|AppendArray (Variables|Default|GetObjectivesSelected) (.Instances (CallFunction|CreateInstanceandLocationArrays (LocalVariables|GetCurrentHitItems) (Utilities|Array|Get(acopy) (Variables|Default|GetZonesObjectivesReversed) _array_index) (.HitComponent (Collision|BreakHitResult (Utilities|Array|Get(acopy) (Variables|Default|GetCurrentResults)))))))
              (Utilities|Struct|SetmembersinST_ZoneLocs (Utilities|Array|Get(acopy) _objectivelocations_2 _array_index) (.Locations (CallFunction|CreateInstanceandLocationArrays (LocalVariables|GetCurrentHitItems) (Utilities|Array|Get(acopy) (Variables|Default|GetZonesObjectivesReversed) _array_index) (.HitComponent (Collision|BreakHitResult (Utilities|Array|Get(acopy) (Variables|Default|GetCurrentResults)))))) (.Available (CallFunction|CreateInstanceandLocationArrays (LocalVariables|GetCurrentHitItems) (Utilities|Array|Get(acopy) (Variables|Default|GetZonesObjectivesReversed) _array_index) (.HitComponent (Collision|BreakHitResult (Utilities|Array|Get(acopy) (Variables|Default|GetCurrentResults)))))))
              (Utilities|Array|Add _radiuslocations_2 _array_element))
            ;[1 1 1] Pass results with Event Dispatcher to GameMode
            (Utilities|Array|Reverse _radiuslocations)
            (Utilities|Array|Reverse _objectivelocations)
            (for _array_element_5 (.ObjectiveLocations (Utilities|Struct|BreakST_ScanningZoneResult (Variables|Default|GetScanningZoneResults)))
              (for _array_element_6 (.Locs (Utilities|Struct|BreakST_ZoneLocs _array_element_5))
                (Development|PrintString (Utilities|String|ToString(Vector) _array_element_6) false true "(R=1.000000,G=0.839822,B=0.000000,A=1.000000)" 5.0)))
            (Default|CallFoundResult (Variables|Default|GetScanningZoneResults))
            (elif (> (LocalVariables|GetAttempts) (Variables|Default|GetFailAttemptsBeforeTryAgain))
              ;[1 1 1] Failed generating, continue searching
              (CallFunction|PendingGenerate)
              (Development|PrintString (Utilities|String|Append "Failed " (Utilities|String|ToString(Integer) (Variables|Default|GetFailAttemptsBeforeTryAgain)) " times:  try again...") _dev_2 _dev_2 "(R=1.000000,G=0.401145,B=0.000000,A=1.000000)")
              (else
                (goto _label)))))))))

(fn CreateInstanceandLocationArrays
  (params (HitIndexes :type Array%20of%20Integers) (TargetAmount :type Integer) (InputPin :type Object%20Object%20Reference))
  (for _index (range 0 (- TargetAmount 1))
    (bind _asfoliage_instanced_static_mesh_component (Utilities|Casting|CastToFoliageInstancedStaticMeshComponent InputPin))
    (Utilities|Array|Add (LocalVariables|GetLocsToBeAdded) (.Location (Math|Transform|BreakTransform (.OutInstanceTransform (Components|InstancedStaticMesh|GetInstanceTransform _asfoliage_instanced_static_mesh_component (Utilities|Array|Get(acopy) HitIndexes _index) true)))))
    (Utilities|Array|Add (LocalVariables|GetAvailableAdded) true))
  ;[1 1 1] Result arrays
  (return (LocalVariables|GetInstancesToBeAdded) (LocalVariables|GetLocsToBeAdded) (LocalVariables|GetAvailableAdded)))

(fn DebugZones
  (params (DrawTime :type Float%20%28single-precision%29))
  (bind _returnvalue (Math|Random|RandomFloat))
  (bind _returnvalue_2 (Math|Random|RandomFloat))
  (bind _returnvalue_3 (Math|Random|RandomFloat))
  (bind _returnvalue_4 (Math|Color|MakeColor _returnvalue _returnvalue_2 _returnvalue_3))
  (for (_array_element _array_index) (Variables|Default|GetFoundZoneLocs)
    (Collision|MultiSphereTraceByChannel (.Start (CallFunction|GetSphereTraceLocs _array_element)) (.End (CallFunction|GetSphereTraceLocs _array_element)) (Math|Conversions|ToFloat(Integer) (Utilities|Array|Get(acopy) (Variables|Default|GetZonesRadius) _array_index)) "TraceTypeQuery3" true 0 "ForDuration" true _returnvalue_4 _returnvalue_4 DrawTime)))

(fn GetSphereTraceLocs
  (params (A :type Vector))
  (return (- A "0, 0,1200.000000") (+ A "0, 0,1200.000000")))

(fn SetupandStartGenerating
  (params (Zones :type Array%20of%20ST%20Scanner%20Zones%20Structures))
  (Utilities|Array|SetArrayElem :TargetArray (LocalVariables|GetObjectiveLocs) :Index (Utilities|Array|LastIndex Zones) :bSizeToFit true)
  (Utilities|Struct|SetmembersinST_ScanningZoneResult (Variables|Default|GetScanningZoneResults) (Utilities|Array|MakeArray "0, 0, 0") (LocalVariables|GetObjectiveLocs))
  (Utilities|Array|Clear (Variables|Default|GetZonesAmountOfObjectives))
  (Utilities|Array|Clear (Variables|Default|GetZonesRadius))
  (for _array_element Zones
    (Utilities|Array|Add (Variables|Default|GetZonesRadius) (.ZoneRadius (Utilities|Struct|BreakST_ScannerZones _array_element)))
    (Utilities|Array|Add (Variables|Default|GetZonesAmountOfObjectives) (.AmountOfBonusObjects (Utilities|Struct|BreakST_ScannerZones _array_element))))
  (CallFunction|GenerateRandomZones))