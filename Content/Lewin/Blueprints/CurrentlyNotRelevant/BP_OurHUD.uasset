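; BP_OurHUD is a HUD Blueprint that creates the in-game WB_GameUI widget and then calls Setup on the BP_OurPC player controller.
; On BeginPlay it creates the UI with the join animation if the controller skips the main menu or the instance is not the server.
; Otherwise creation waits for the CreateGameUi event, which shows the UI without that animation and runs the same controller setup.
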(event Custom|CreateGameUi
  (bind _returnvalue (UserInterface|CreateWidget "/Game/Lewin/UI/WB_GameUI.WB_GameUI_C" 0 false))
  (bind _output_get (Variables|Default|SetGameUI _returnvalue))
  (UserInterface|Viewport|AddtoViewport _output_get 0)
  ;[1 1 1] Create GameUI
  (bind _asbp_our_pc (Utilities|Casting|CastToBP_OurPC (Game|GetPlayerController 0)))
  (Default|Setup _asbp_our_pc))

(event EventBeginPlay
  (bind _asbp_our_pc (Utilities|Casting|CastToBP_OurPC (Game|GetPlayerController 0)))
  (if (Variables|/Game/Lewin/Blueprints/BP_OurPC.BP_OurPC_C|GetSKIP_MainMenu _asbp_our_pc)
    ;[1 1 1] Create GameUI
    (bind _returnvalue (UserInterface|CreateWidget "/Game/Lewin/UI/WB_GameUI.WB_GameUI_C" :!label _label))
    (bind _output_get (Variables|Default|SetGameUI _returnvalue))
    (UserInterface|Viewport|AddtoViewport _output_get 0)
    (bind _asbp_our_pc_2 (Utilities|Casting|CastToBP_OurPC (Game|GetPlayerController 0)))
    (Default|Setup _asbp_our_pc_2)
    (elif (not (Networking|IsServer))
      (goto _label))))

(fn ConstructionScript)