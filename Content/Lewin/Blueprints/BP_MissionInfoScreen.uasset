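; BP_MissionInfoScreen is an in-world screen that displays mission info and a final mission summary through a WB_MissionInfo widget component.
; Events set replicated variables for power, live data and finished-mission data, whose RepNotify functions toggle visibility and forward data to the widget.
; The final screen redraws every frame while shown; hiding it resets the widget and throttles redraw to once per second.
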(event Custom|TurnOn
  (params (On :type Boolean))
  (Variables|Default|SetTurnON_Server On))

(event Custom|Update
  (params (Data :type ST%20Update%20Info%20Screen%20Structure))
  (Variables|Default|SetData Data))

(event Custom|ShowFinalScreen
  (params (FinishedMissionData :type ST%20Finished%20Mission%20Structure))
  (Variables|Default|SetFinishedMissionData FinishedMissionData))

(fn ConstructionScript)

(fn OnRepTurnONServer
  (Rendering|SetVisibility (Variables|Default|GetScreenWidget) (Variables|Default|GetTurnON_Server) false))

(fn OnRepData
  (bind _aswb_mission_info (Utilities|Casting|CastToWB_MissionInfo (UserInterface|GetUserWidgetObject (Variables|Default|GetScreenWidget))))
  (Default|Update _aswb_mission_info (Variables|Default|GetData)))

(fn OnRepFinishedMissionData
  (if (Utilities|Struct|BreakST_FinishedMission (Variables|Default|GetFinishedMissionData))
    (Class|WidgetComponent|SetRedrawTime (Variables|Default|GetScreenWidget) 0.0)
    (bind _aswb_mission_info (Utilities|Casting|CastToWB_MissionInfo (UserInterface|GetUserWidgetObject (Variables|Default|GetScreenWidget))))
    (Default|ShowFinalScreen _aswb_mission_info (Variables|Default|GetFinishedMissionData))
    (else
      (bind _aswb_mission_info_2 (Utilities|Casting|CastToWB_MissionInfo (UserInterface|GetUserWidgetObject (Variables|Default|GetScreenWidget))))
      (Default|Reset _aswb_mission_info_2)
      (Class|WidgetComponent|SetRedrawTime (Variables|Default|GetScreenWidget) 1.0))))