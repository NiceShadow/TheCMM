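; Mission zone actor that bounds the local player's play area and hosts a movable scan zone for scanner rovers.
; An inner cylinder fades the border in as the player nears it, while the visible cylinder starts or cancels the controller's out-of-zone handling.
; The server tells the game mode whether scanning is allowed, and replicated Activate toggles collision.
; The construction script grid-snaps cylinder scales and places dev coordinate labels.
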(event OnComponentBeginOverlap(CylinderOverlap)
  (params (OverlappedComponent :type Primitive%20Component%20Object%20Reference) (OtherActor :type Actor%20Object%20Reference) (OtherComp :type Primitive%20Component%20Object%20Reference) (OtherBodyIndex :type Integer) (bFromSweep :type Boolean) (SweepResult :type Hit%20Result%20Structure%20%28by%20ref%29))
  ;[1 1 1] Trigger show hide mission zone before actual border
  (if (== OtherActor (Game|Player|GetPlayerPawn 0))
    (CallFunction|ShowMissionZone false)))

(event OnComponentEndOverlap(CylinderOverlap)
  (params (OverlappedComponent :type Primitive%20Component%20Object%20Reference) (OtherActor :type Actor%20Object%20Reference) (OtherComp :type Primitive%20Component%20Object%20Reference) (OtherBodyIndex :type Integer))
  ;[1 1 1] Trigger show hide mission zone before actual border
  (if (== OtherActor (Game|Player|GetPlayerPawn 0))
    (CallFunction|ShowMissionZone true)))

(event OnComponentBeginOverlap(CylinderShow)
  (params (OverlappedComponent :type Primitive%20Component%20Object%20Reference) (OtherActor :type Actor%20Object%20Reference) (OtherComp :type Primitive%20Component%20Object%20Reference) (OtherBodyIndex :type Integer) (bFromSweep :type Boolean) (SweepResult :type Hit%20Result%20Structure%20%28by%20ref%29))
  ;[1 1 1] Trigger leaving/entering zone
  (if (== OtherActor (Game|Player|GetPlayerPawn 0))
    (bind _asbp_our_pc (Utilities|Casting|CastToBP_OurPC (Game|GetPlayerController 0)))
    (Default|StartOutOfZone _asbp_our_pc false true "0, 0, 0" 0.0)))

(event OnComponentEndOverlap(CylinderShow)
  (params (OverlappedComponent :type Primitive%20Component%20Object%20Reference) (OtherActor :type Actor%20Object%20Reference) (OtherComp :type Primitive%20Component%20Object%20Reference) (OtherBodyIndex :type Integer))
  ;[1 1 1] Trigger leaving/entering zone
  (if (== OtherActor (Game|Player|GetPlayerPawn 0))
    (bind _asbp_our_pc (Utilities|Casting|CastToBP_OurPC (Game|GetPlayerController 0)))
    (Default|StartOutOfZone _asbp_our_pc true true (Transformation|GetActorLocation) (Variables|Default|GetZeroDistance))))

(event OnComponentBeginOverlap(CylinderScanningScannerZone)
  (params (OverlappedComponent :type Primitive%20Component%20Object%20Reference) (OtherActor :type Actor%20Object%20Reference) (OtherComp :type Primitive%20Component%20Object%20Reference) (OtherBodyIndex :type Integer) (bFromSweep :type Boolean) (SweepResult :type Hit%20Result%20Structure%20%28by%20ref%29))
  (bind _lastscanzone (Variables|Default|GetLastScanZone))
  (bind _returnvalue (not _lastscanzone))
  ;[1 1 1] Server Trigger if scanning rover enters zone to scan
  (Networking|SwitchHasAuthority
    (:Authority
      (bind _asparent_rover (Utilities|Casting|CastToParentRover OtherActor))
      (if (Utilities|Enum|Equal(Enum) (Variables|/Game/CustomVehicle/ParentRover.ParentRover_C|GetRoverType _asparent_rover) "NewEnumerator2")
        (bind _asbp_our_gm (Utilities|Casting|CastToBP_OurGM (Game|GetGameMode)))
        (Default|UpdateRoverCanScan _asbp_our_gm _asparent_rover _returnvalue)
        (bind _output_get (Variables|Default|SetScannerCanScan _returnvalue))
        (if _output_get
          (Variables|Default|SetCurrentScannerRoverInZone _asparent_rover))))))

(event OnComponentEndOverlap(CylinderScanningScannerZone)
  (params (OverlappedComponent :type Primitive%20Component%20Object%20Reference) (OtherActor :type Actor%20Object%20Reference) (OtherComp :type Primitive%20Component%20Object%20Reference) (OtherBodyIndex :type Integer))
  ;[1 1 1] Server Trigger if scanning rover enters zone to scan
  (Networking|SwitchHasAuthority
    (:Authority
      (bind _asparent_rover (Utilities|Casting|CastToParentRover OtherActor))
      (if (Utilities|Enum|Equal(Enum) (Variables|/Game/CustomVehicle/ParentRover.ParentRover_C|GetRoverType _asparent_rover) "NewEnumerator2")
        (Variables|Default|SetCurrentScannerRoverInZone 0)
        (bind _asbp_our_gm (Utilities|Casting|CastToBP_OurGM (Game|GetGameMode)))
        (Default|UpdateRoverCanScan _asbp_our_gm _asparent_rover false)
        (Variables|Default|SetScannerCanScan false)))))

(event Custom|ShowMissionZone
  (params (In :type Boolean))
  ;[1 1 1] Show Mission zone border animated locally
  (if In
    (Development|SetHiddeninGame (Variables|Default|GetCylinderShow) false false)
    (CallFunction|SetupInstanceMATifNeeded)
    (bind _newtrack_0 (Timeline|Timeline_0 Play)
      (:Update
        (Rendering|Material|SetScalarParameterValue (Variables|Default|GetZoneInstanceMAT) "Opacity" _newtrack_0 :!class /Script/Engine.MaterialInstanceDynamic))
      (:Finished
        (if (not In)
          (Development|SetHiddeninGame (Variables|Default|GetCylinderShow) true false))))
    (else
      (CallFunction|SetupInstanceMATifNeeded)
      (Timeline|Timeline_0 Reverse))))

(event Custom|ActivateOnServer
  (params (Activate :type Boolean))
  ;[1 1 1] Activate this Mission zone actor
  (Variables|Default|SetActivate Activate))

(event Custom|ShowMissionZoneInstant
  (params (Show :type Boolean))
  ;[1 1 1] Show Mission zone border animated locally
  ;;[1 1 1 1 30] show instant
  (Development|SetHiddeninGame (Variables|Default|GetCylinderShow) (not Show) false))

(event Custom|SetZoneToScanLocation
  (params (CurrentScanLocation :type Vector) (Last :type Boolean))
  (bind _scanradius (Variables|Default|GetScanRadius))
  (bind _cylinderscanningscannerzone (Variables|Default|GetCylinderScanningScannerZone))
  (bind _returnvalue (/ _scanradius 5e+01))
  ;[1 1 1] Update scanning zone location and scale on server
  (Transformation|SetWorldLocation _cylinderscanningscannerzone CurrentScanLocation false false)
  (Variables|Default|SetLastScanZone Last)
  (Transformation|SetWorldScale3D _cylinderscanningscannerzone (Math|Vector|MakeVector _returnvalue _returnvalue 2e+02))
  (Utilities|IsValid (Variables|Default|GetCurrentScannerRoverInZone)
    (:Is%20Valid
      (if (Variables|Default|GetLastScanZone)
        (bind _asbp_our_gm (Utilities|Casting|CastToBP_OurGM (Game|GetGameMode)))
        (Variables|Default|SetScannerCanScan false)
        (Default|UpdateRoverCanScan _asbp_our_gm (Variables|Default|GetCurrentScannerRoverInZone) false)
        (Variables|Default|SetCurrentScannerRoverInZone 0)
        (else
          (bind _asbp_our_gm_2 (Utilities|Casting|CastToBP_OurGM (Game|GetGameMode)))
          (bind _output_get (Variables|Default|SetScannerCanScan (Collision|IsOverlappingActor (Variables|Default|GetCylinderScanningScannerZone) (Variables|Default|GetCurrentScannerRoverInZone) :!class /Script/Engine.PrimitiveComponent)))
          (Default|UpdateRoverCanScan _asbp_our_gm_2 (Variables|Default|GetCurrentScannerRoverInZone) _output_get)
          (if (not (Variables|Default|GetScannerCanScan))
            (Variables|Default|SetCurrentScannerRoverInZone 0)))))))

(event EventBeginPlay
  ;[1 1 1] Setup
  (if (Variables|Default|GetUseScanningZone)
    (Rendering|SetVisibility (Variables|Default|GetCylinderScanningFirstZone) false false)
    (else
      (Components|DestroyComponent (Variables|Default|GetCylinderScanningFirstZone))))
  (if (not (Variables|Default|GetDevView))
    (Components|DestroyComponent (Variables|Default|GetTextRenderX))))

(fn ConstructionScript
  (bind _coordinatedivider (Variables|Default|GetCoordinateDivider))
  (bind _coordinatedivider_2 (Variables|Default|GetCoordinateDivider))
  (bind _coordinatedivider_3 (Variables|Default|GetCoordinateDivider))
  (bind _coordinatedivider_4 (Variables|Default|GetCoordinateDivider))
  (bind _scanningzonestartradius (Variables|Default|GetScanningZoneStartRadius))
  (bind _cylindershow (Variables|Default|GetCylinderShow))
  (bind _textrenderx (Variables|Default|GetTextRenderX))
  (bind _textrendery (Variables|Default|GetTextRenderY))
  (bind _distanceoverlapandvisualborder (Variables|Default|GetDistanceOverlapAndVisualBorder))
  (bind _textrendernx (Variables|Default|GetTextRenderNX))
  (bind _returnvalue (Math|Conversions|ToVector(Float) _distanceoverlapandvisualborder))
  (bind _returnvalue_2 (Transformation|GetWorldLocation _textrendernx))
  (bind _returnvalue_3 (Math|Conversions|ToFloat(Integer) _coordinatedivider_4))
  (bind _returnvalue_4 (/ _scanningzonestartradius 5e+01))
  (bind _returnvalue_5 (Transformation|GetWorldScale _cylindershow))
  (bind _returnvalue_6 (Transformation|GetWorldLocation _textrenderx))
  (bind _returnvalue_7 (Transformation|GetWorldLocation _textrendery))
  (bind _x (Math|Vector|BreakVector _returnvalue_2))
  (bind _x_2 (Math|Vector|BreakVector _returnvalue_6))
  (bind _y (Math|Vector|BreakVector _returnvalue_7))
  (bind _returnvalue_8 (Class|KismetMathLibrary|VectorSnappedtoGrid _returnvalue_5 _returnvalue_3))
  (bind _returnvalue_9 (- _returnvalue_8 _returnvalue))
  (bind _returnvalue_10 (Math|Float|SnapToGrid(Float) _x_2 1e+03))
  (bind _returnvalue_11 (Math|Float|SnapToGrid(Float) _x 1e+03))
  (bind _returnvalue_12 (Math|Float|SnapToGrid(Float) _y 1e+03))
  (bind _returnvalue_13 (Math|Float|Truncate _returnvalue_11))
  (bind _returnvalue_14 (Math|Float|Truncate _returnvalue_10))
  (bind _returnvalue_15 (Math|Float|Truncate _returnvalue_12))
  (bind _returnvalue_16 (/ _returnvalue_13 _coordinatedivider_3))
  (bind _returnvalue_17 (/ _returnvalue_14 _coordinatedivider))
  (bind _returnvalue_18 (/ _returnvalue_15 _coordinatedivider_2))
  ;[1 1 1] Setup scales
  (Transformation|SetWorldScale3D (Variables|Default|GetCylinderShow) _returnvalue_8)
  (Transformation|SetWorldScale3D (Variables|Default|GetCylinderOverlap) _returnvalue_9)
  (Variables|Default|SetZeroDistance (* (.X (Math|Vector|BreakVector _returnvalue_8)) 5e+01))
  (Transformation|SetWorldScale3D (Variables|Default|GetCylinderScanningFirstZone) (Math|Vector|MakeVector _returnvalue_4 _returnvalue_4 (.Z (Math|Vector|BreakVector _returnvalue_9))))
  (if (Variables|Default|GetDevView)
    (Rendering|SetVisibility (Variables|Default|GetTextRenderX) true false)
    (Rendering|SetVisibility (Variables|Default|GetCylinderScanningFirstZone) (Variables|Default|GetUseScanningZone) false)
    ;[1 1 1] Dev Text Info
    (Transformation|SetWorldLocation (Variables|Default|GetTextRenderX) (+ (Transformation|GetActorLocation) (Math|Vector|MakeVector (Variables|Default|GetZeroDistance) 0.0 0.0)) false false)
    (Transformation|SetWorldLocation (Variables|Default|GetTextRenderX_Info) (- (+ (Transformation|GetActorLocation) (Math|Vector|MakeVector (Variables|Default|GetZeroDistance) 0.0 0.0)) "-10.000000, 0,100.000000") false false)
    (Rendering|Components|TextRender|SetText (Variables|Default|GetTextRenderX) (Utilities|Text|ToText(Integer) _returnvalue_17))
    (Variables|Default|SetStartX _returnvalue_17)
    (Transformation|SetWorldLocation (Variables|Default|GetTextRenderNX) (+ (Transformation|GetActorLocation) (Math|Vector|MakeVector (* (Variables|Default|GetZeroDistance) -1.0) 0.0 0.0)) false false)
    (Rendering|Components|TextRender|SetText (Variables|Default|GetTextRenderNX) (Utilities|Text|ToText(Integer) _returnvalue_16))
    (Transformation|SetWorldLocation (Variables|Default|GetTextRenderY) (+ (Transformation|GetActorLocation) (Math|Vector|MakeVector 0.0 (* (Variables|Default|GetZeroDistance) -1.0) 0.0)) false false)
    (Rendering|Components|TextRender|SetText (Variables|Default|GetTextRenderY) (Utilities|Text|ToText(Integer) _returnvalue_18))
    (Variables|Default|SetStartY _returnvalue_18)
    (Variables|Default|SetEndX _returnvalue_16)
    (LocalVariables|SetTotalXDistance (Math|Integer|Absolute(Integer) (- _returnvalue_17 _returnvalue_16)))
    (Rendering|Components|TextRender|SetText (Variables|Default|GetTextRenderX_Info) (Utilities|Text|ToText(String) (Utilities|String|Append (Utilities|String|ToString(Integer) (LocalVariables|GetTotalXDistance)) "____" "5x " (Utilities|String|ToString(Integer) (/ (LocalVariables|GetTotalXDistance) 4)) ";  " "7x " (Utilities|String|ToString(Integer) (/ (LocalVariables|GetTotalXDistance) 6)) ";  " "9x " (Utilities|String|ToString(Integer) (/ (LocalVariables|GetTotalXDistance) 8)))))))

(fn SetupInstanceMATifNeeded
  (Utilities|IsValid (Variables|Default|GetZoneInstanceMAT)
    (:Is%20Not%20Valid
      (bind _returnvalue (Rendering|Material|CreateDynamicMaterialInstance "/Game/Lewin/Blueprints/TestMaterials/M_MissionZoneShow_Inst.M_MissionZoneShow_Inst" "None" "None" :!class /Script/Engine.KismetMaterialLibrary))
      (bind _output_get (Variables|Default|SetZoneInstanceMAT _returnvalue))
      (Rendering|Material|SetMaterial (Variables|Default|GetCylinderShow) 0 _output_get))))

(fn OnRepActivate
  (Collision|SetCollisionEnabled (Variables|Default|GetCylinderOverlap) (select (Variables|Default|GetActivate) "QueryAndPhysics" "NoCollision")))