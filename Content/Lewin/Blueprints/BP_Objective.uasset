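; BP_Objective is a physics-driven objective object whose mesh comes from the row in the Objectives data table matching its ID.
; On BeginPlay it launches the cube upward, enables blocking against the Destructible channel after a short delay, and hands the cube to SmoothSync for syncing.
; EnableReturnable opens a two-second Returnable window, whose RepNotify toggles BoxHover query collision and turns on cube physics when opened.
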(event Custom|EnableReturnable
  (Variables|Default|SetReturnable true)
  (Utilities|FlowControl|Delay 2.0)
  (Variables|Default|SetReturnable false))

(event EventBeginPlay
  (bind _out_row (CallFunction|GetDatabyID))
  (Variables|Default|SetData _out_row)
  (Components|StaticMesh|SetStaticMesh (Variables|Default|GetCube) (.Mesh (Utilities|Struct|BreakST_Objective (Variables|Default|GetData))))
  ;[1 1 1] Add inital impulse
  (Physics|AddImpulse (Variables|Default|GetCube) (Math|Vector|MakeVector 0.0 0.0 5e+04) "None" false)
  (Utilities|FlowControl|Delay 0.5)
  (Collision|SetCollisionResponsetoChannel (Variables|Default|GetCube) "ECC_Destructible" "ECR_Block")
  (Class|SmoothSync|SetSceneComponenttoSync (Variables|Default|GetSmoothSync) (Variables|Default|GetCube)))

(fn ConstructionScript)

(fn GetDatabyID
  (bind _outrownames (DataTable|GetDataTableRowNames "/Game/Balduin/Objectives.Objectives"))
  (for _array_element _outrownames
    (bind _returnvalue (Utilities|GetDataTableRow "/Game/Balduin/Objectives.Objectives" _array_element)
      (:then
        (if (== (Variables|Default|GetID) (Utilities|Struct|BreakST_Objective _returnvalue))
          (return _returnvalue))))))

(fn OnRepSyncActivated)

(fn OnRepReturnable
  (if (Variables|Default|GetReturnable)
    (Collision|SetCollisionEnabled (Variables|Default|GetBoxHover) "QueryOnly")
    (Development|PrintString "BRA")
    (Physics|SetSimulatePhysics (Variables|Default|GetCube) true)
    (else
      (Collision|SetCollisionEnabled (Variables|Default|GetBoxHover) "NoCollision"))))