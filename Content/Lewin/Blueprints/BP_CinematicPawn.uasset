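; BP_CinematicPawn is a cinematic camera pawn with live tuning of movement speed and spring-arm lag.
; Holding G, H or J while scrolling adjusts custom time dilation (as speed), lag or rotation lag, echoed to the cine UI through BP_OurPC.
; Rotation lag writes to CameraLagSpeed, like lag, and toggles EnableCameraRotationLag by sign.
; F toggles the cine UI and K toggles terrain light on the player controller.
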(event Input|MouseEvents|MouseWheelDown
  (params (Key :type Key%20Structure :default "None"))
  (:Pressed
    (if (Variables|Default|GetPressG)
      (Variables|Default|SetSpeed (+ (Variables|Default|GetSpeed) -0.2))
      (Variables|Default|SetCustomTimeDilation (Math|Float|Clamp(Float) (Variables|Default|GetSpeed) 0.3 (Variables|Default|GetSpeed)))
      (bind _asbp_our_pc (Utilities|Casting|CastToBP_OurPC (Game|GetPlayerController 0)))
      (Rendering|Components|TextRender|SetText (Variables|/Game/Lewin/WB_CineUI.WB_CineUI_C|GetSp (Variables|/Game/Lewin/UI/WB_GameUI.WB_GameUI_C|GetWB_CineUI (Variables|/Game/Lewin/Blueprints/BP_OurPC.BP_OurPC_C|GetGameUI_Ref _asbp_our_pc))) (Utilities|Text|ToText(Float) (Variables|Default|GetSpeed) "HalfToEven" false true 1 20 0 1))
      (elif (Variables|Default|GetPressH)
        (Variables|Default|SetLag (+ (Variables|Default|GetLag) -0.2))
        (Variables|/Script/Engine.SpringArmComponent|SetCameraLagSpeed (Variables|Default|GetSpringArm) (Math|Float|Clamp(Float) (Variables|Default|GetLag) 0.0 (Variables|Default|GetLag)))
        (bind _asbp_our_pc_2 (Utilities|Casting|CastToBP_OurPC (Game|GetPlayerController 0)))
        (Rendering|Components|TextRender|SetText (Variables|/Game/Lewin/WB_CineUI.WB_CineUI_C|GetlagT (Variables|/Game/Lewin/UI/WB_GameUI.WB_GameUI_C|GetWB_CineUI (Variables|/Game/Lewin/Blueprints/BP_OurPC.BP_OurPC_C|GetGameUI_Ref _asbp_our_pc_2))) (Utilities|Text|ToText(Float) (Variables|Default|GetLag) "HalfToEven" false true 1 20 0 1))
        (elif (Variables|Default|GetTR)
          (Variables|Default|SetRLag (+ (Variables|Default|GetRLag) -0.2))
          (Variables|/Script/Engine.SpringArmComponent|SetCameraLagSpeed (Variables|Default|GetSpringArm) (Math|Float|Clamp(Float) (Variables|Default|GetRLag) 0.0 (Variables|Default|GetRLag)))
          (Variables|/Script/Engine.SpringArmComponent|SetbEnableCameraRotationLag (Variables|Default|GetSpringArm) (not (< (Variables|Default|GetRLag) 0.0)))
          (bind _asbp_our_pc_3 (Utilities|Casting|CastToBP_OurPC (Game|GetPlayerController 0)))
          (Rendering|Components|TextRender|SetText (Variables|/Game/Lewin/WB_CineUI.WB_CineUI_C|GetlagT_1 (Variables|/Game/Lewin/UI/WB_GameUI.WB_GameUI_C|GetWB_CineUI (Variables|/Game/Lewin/Blueprints/BP_OurPC.BP_OurPC_C|GetGameUI_Ref _asbp_our_pc_3))) (Utilities|Text|ToText(Float) (Variables|Default|GetRLag) "HalfToEven" false true 1 20 0 1)))))))

(event Input|MouseEvents|MouseWheelUp
  (params (Key :type Key%20Structure :default "None"))
  (:Pressed
    (if (Variables|Default|GetPressG)
      (Variables|Default|SetSpeed (+ (Variables|Default|GetSpeed) 0.2))
      (Variables|Default|SetCustomTimeDilation (Math|Float|Clamp(Float) (Variables|Default|GetSpeed) 1.0 (Variables|Default|GetSpeed)))
      (bind _asbp_our_pc (Utilities|Casting|CastToBP_OurPC (Game|GetPlayerController 0)))
      (Rendering|Components|TextRender|SetText (Variables|/Game/Lewin/WB_CineUI.WB_CineUI_C|GetSp (Variables|/Game/Lewin/UI/WB_GameUI.WB_GameUI_C|GetWB_CineUI (Variables|/Game/Lewin/Blueprints/BP_OurPC.BP_OurPC_C|GetGameUI_Ref _asbp_our_pc))) (Utilities|Text|ToText(Float) (Variables|Default|GetSpeed) "HalfToEven" false true 1 20 0 1))
      (elif (Variables|Default|GetPressH)
        (Variables|Default|SetLag (+ (Variables|Default|GetLag) 0.2))
        (Variables|/Script/Engine.SpringArmComponent|SetCameraLagSpeed (Variables|Default|GetSpringArm) (Math|Float|Clamp(Float) (Variables|Default|GetLag) 0.0 (Variables|Default|GetLag)))
        (bind _asbp_our_pc_2 (Utilities|Casting|CastToBP_OurPC (Game|GetPlayerController 0)))
        (Rendering|Components|TextRender|SetText (Variables|/Game/Lewin/WB_CineUI.WB_CineUI_C|GetlagT (Variables|/Game/Lewin/UI/WB_GameUI.WB_GameUI_C|GetWB_CineUI (Variables|/Game/Lewin/Blueprints/BP_OurPC.BP_OurPC_C|GetGameUI_Ref _asbp_our_pc_2))) (Utilities|Text|ToText(Float) (Variables|Default|GetLag) "HalfToEven" false true 1 20 0 1))
        (elif (Variables|Default|GetTR)
          (Variables|Default|SetRLag (+ (Variables|Default|GetRLag) 0.2))
          (Variables|/Script/Engine.SpringArmComponent|SetCameraLagSpeed (Variables|Default|GetSpringArm) (Math|Float|Clamp(Float) (Variables|Default|GetRLag) 0.0 (Variables|Default|GetRLag)))
          (Variables|/Script/Engine.SpringArmComponent|SetbEnableCameraRotationLag (Variables|Default|GetSpringArm) (not (< (Variables|Default|GetRLag) 0.0)))
          (bind _asbp_our_pc_3 (Utilities|Casting|CastToBP_OurPC (Game|GetPlayerController 0)))
          (Rendering|Components|TextRender|SetText (Variables|/Game/Lewin/WB_CineUI.WB_CineUI_C|GetlagT_1 (Variables|/Game/Lewin/UI/WB_GameUI.WB_GameUI_C|GetWB_CineUI (Variables|/Game/Lewin/Blueprints/BP_OurPC.BP_OurPC_C|GetGameUI_Ref _asbp_our_pc_3))) (Utilities|Text|ToText(Float) (Variables|Default|GetRLag) "HalfToEven" false true 1 20 0 1)))))))

(event Input|KeyboardEvents|F
  (params (Key :type Key%20Structure :default "None"))
  (:Pressed
    (bind _asbp_our_pc (Utilities|Casting|CastToBP_OurPC (Game|GetPlayerController 0)))
    (Widget|SetVisibility (Variables|/Game/Lewin/UI/WB_GameUI.WB_GameUI_C|GetWB_CineUI (Variables|/Game/Lewin/Blueprints/BP_OurPC.BP_OurPC_C|GetGameUI_Ref _asbp_our_pc)) (select (Widget|IsVisible (Variables|/Game/Lewin/UI/WB_GameUI.WB_GameUI_C|GetWB_CineUI (Variables|/Game/Lewin/Blueprints/BP_OurPC.BP_OurPC_C|GetGameUI_Ref _asbp_our_pc))) "Collapsed" "HitTestInvisible"))))

(event Input|KeyboardEvents|G
  (params (Key :type Key%20Structure :default "None"))
  (:Pressed
    (Variables|Default|SetPressG true))
  (:Released
    (Variables|Default|SetPressG false)))

(event Input|KeyboardEvents|H
  (params (Key :type Key%20Structure :default "None"))
  (:Pressed
    (Variables|Default|SetPressH true))
  (:Released
    (Variables|Default|SetPressH false)))

(event Input|KeyboardEvents|K
  (params (Key :type Key%20Structure :default "None"))
  (:Pressed
    (Variables|Default|SetTL (not (Variables|Default|GetTL)))
    (bind _asbp_our_pc (Utilities|Casting|CastToBP_OurPC (Game|GetPlayerController 0)))
    (Default|ToggleTerrainLight _asbp_our_pc (Variables|Default|GetTL))))

(event Input|KeyboardEvents|J
  (params (Key :type Key%20Structure :default "None"))
  (:Pressed
    (Variables|Default|SetTR true))
  (:Released
    (Variables|Default|SetTR false)))

(fn ConstructionScript)